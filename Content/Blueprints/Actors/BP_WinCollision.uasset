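; BP_WinCollision is a level-exit trigger that completes the level when the player overlaps its box and no BP_Crystal actors remain.
; It finds the current map in a Levels array, shows WBP_WinningMessage, then after a delay opens the next level or quits on the final one.
; If crystals remain, it briefly shows a collect-all message, using a resettable DoOnce to prevent stacked widgets.
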(event OnComponentBeginOverlap(Box)
  (params (OverlappedComponent :type Primitive%20Component%20Object%20Reference) (OtherActor :type Actor%20Object%20Reference) (OtherComp :type Primitive%20Component%20Object%20Reference) (OtherBodyIndex :type Integer) (bFromSweep :type Boolean) (SweepResult :type Hit%20Result%20Structure%20%28by%20ref%29))
  (Utilities|IsPlayer? OtherActor
    (:IsPlayer
      (bind _outactors (Actor|GetAllActorsOfClass "/Game/Blueprints/Actors/BP_Crystal.BP_Crystal_C"))
      (if (== (Utilities|Array|Length _outactors) 0)
        (if (CallFunction|IsFinalLevel)
          (Variables|Default|SetWinningMessage (Utilities|Text|ToText(String) (Utilities|String|Append "Level " (Utilities|String|ToString(Integer) (+ (CallFunction|FindCurrentLevel) 1)) " Complete")))
          (bind _returnvalue (UserInterface|CreateWidget "/Game/Blueprints/Widgets/WBP_WinningMessage.WBP_WinningMessage_C"))
          (UserInterface|Viewport|AddtoViewport _returnvalue 0)
          (Utilities|FlowControl|Delay 2.5)
          (Game|QuitGame 0 "Quit" false)
          (else
            (Variables|Default|SetWinningMessage (Utilities|Text|ToText(String) (Utilities|String|Append "Level " (Utilities|String|ToString(Integer) (+ (CallFunction|FindCurrentLevel) 1)) " Complete")))
            (bind _returnvalue_2 (UserInterface|CreateWidget "/Game/Blueprints/Widgets/WBP_WinningMessage.WBP_WinningMessage_C"))
            (UserInterface|Viewport|AddtoViewport _returnvalue_2 0)
            (Utilities|FlowControl|Delay 2.5)
            (Game|OpenLevel(byName) (Utilities|Array|Get(acopy) (Variables|Default|GetLevels) (+ (CallFunction|FindCurrentLevel) 1)))))
        (else
          (Utilities|FlowControl|DoOnce false :!label _label
            (:Completed
              (bind _returnvalue_3 (UserInterface|CreateWidget "/Game/Blueprints/Widgets/WBP_WinningMessage.WBP_WinningMessage_C"))
              (UserInterface|Viewport|AddtoViewport _returnvalue_3 0)
              (Variables|Default|SetWinningMessage (Utilities|Text|ToText(String) (Utilities|String|Append "all crystals must " "be collected")))
              (Utilities|FlowControl|Delay 3.0)
              (Widget|RemovefromParent _returnvalue_3)
              (goto _label Reset))))))))

(event EventBeginPlay)

(event Collision|EventActorBeginOverlap
  (params (OtherActor :type Actor%20Object%20Reference)))

(event EventTick
  (params (DeltaSeconds :type Float%20%28single-precision%29)))

(fn ConstructionScript)

(fn FindCurrentLevel
  (bind _returnvalue (Game|GetCurrentLevelName true))
  (return (Utilities|Array|FindItem (Variables|Default|GetLevels) (Utilities|String|StringToName _returnvalue))))

(fn IsFinalLevel
  (return (== (CallFunction|FindCurrentLevel) (Utilities|Array|LastIndex (Variables|Default|GetLevels)))))