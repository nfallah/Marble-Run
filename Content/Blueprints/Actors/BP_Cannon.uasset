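; BP_Cannon is an actor that automatically and repeatedly fires BP_ProJectile from the moment play begins.
; A looping Delay on BeginPlay sets the interval from ShotsPerSecond, with no use of Tick.
; Each cycle restarts the CannonFire timeline to move the Cannon component along local Y and spawns a projectile at the Arrow component's world location and rotation, scaled by BulletScale.
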(event EventBeginPlay
  (bind _arrow (Variables|Default|GetArrow))
  ;[1 1 1] Shots per second
  (Utilities|FlowControl|Delay (/ 1.0 (Variables|CannonOptions|GetShots%20Per%20Second)) :!label _label)
  (Utilities|FlowControl|Sequence
    (:then_0
      ;[1 1 1] Cannon fire animation
      (bind _movecannon (Timeline|CannonFire PlayFromStart)
        (:Update
          (Transformation|SetRelativeLocation (Variables|Default|GetCannon) (Math|Vector|MakeVector 0.0 _movecannon 0.0) false false))))
    (:then_1
      ;[1 1 1] Summon bullet in respect to arrow component
      (Game|SpawnActorfromClass "/Game/Blueprints/Actors/BP_ProJectile.BP_ProJectile_C" (Math|Transform|MakeTransform (Transformation|GetWorldLocation _arrow) (Transformation|GetWorldRotation _arrow) (Math|Conversions|ToVector(Float) (Variables|CannonOptions|GetBullet%20Scale))) "Undefined" 0 0)
      (goto _label))))

(event Collision|EventActorBeginOverlap
  (params (OtherActor :type Actor%20Object%20Reference)))

(event EventTick
  (params (DeltaSeconds :type Float%20%28single-precision%29)))

(fn ConstructionScript)