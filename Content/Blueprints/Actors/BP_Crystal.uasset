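; BP_Crystal is a pickup actor that collects itself when the player overlaps its sphere collision.
; On overlap it caches its location, scale and light intensity, then plays the Collection timeline.
; The timeline's tracks lerp the crystal toward player pawn 0's current location, shrink it to zero and fade PyramidLight, then the actor is destroyed.
; BeginPlay creates and stores a WBP_HUD widget, which is not used further here.
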(event OnComponentBeginOverlap(SphereCollision)
  (params (OverlappedComponent :type Primitive%20Component%20Object%20Reference) (OtherActor :type Actor%20Object%20Reference) (OtherComp :type Primitive%20Component%20Object%20Reference) (OtherBodyIndex :type Integer) (bFromSweep :type Boolean) (SweepResult :type Hit%20Result%20Structure%20%28by%20ref%29))
  (Utilities|IsPlayer? OtherActor
    (:IsPlayer
      (CallFunction|InitializeStartingValues)
      (bind (_direction _move_actor _scale_actor _light_intensity) (Timeline|Collection Play)
        (:Update
          (CallFunction|MovetoPlayerPawn _move_actor)
          (CallFunction|ScaleActortoZero _scale_actor)
          (CallFunction|SetActorIntensity _light_intensity))
        (:Finished
          (Actor|DestroyActor))))))

(event EventBeginPlay
  (bind _returnvalue (UserInterface|CreateWidget "/Game/Blueprints/Widgets/WBP_HUD.WBP_HUD_C"))
  (Variables|Default|SetHUD _returnvalue))

(event Collision|EventActorBeginOverlap
  (params (OtherActor :type Actor%20Object%20Reference)))

(event EventTick
  (params (DeltaSeconds :type Float%20%28single-precision%29)))

(fn ConstructionScript)

(fn MovetoPlayerPawn
  (params (Alpha :type Float%20%28single-precision%29))
  (Transformation|SetActorLocation (Math|Vector|Lerp(Vector) (Variables|Default|GetActorLocation) (Transformation|GetActorLocation (Game|Player|GetPlayerPawn 0)) Alpha) false false))

(fn InitializeStartingValues
  (Variables|Default|SetActorLocation (Transformation|GetActorLocation))
  (Variables|Default|SetActorScale (Transformation|GetActorScale3D))
  (Variables|Default|SetPointLightIntensity (Variables|/Script/Engine.LightComponentBase|GetIntensity (Variables|Default|GetPyramidLight))))

(fn ScaleActortoZero
  (params (Alpha :type Float%20%28single-precision%29))
  (Transformation|SetActorScale3D (Math|Vector|Lerp(Vector) (Variables|Default|GetActorScale) "0, 0, 0" Alpha)))

(fn SetActorIntensity
  (params (Alpha :type Float%20%28single-precision%29))
  (Rendering|Components|Light|SetIntensity (Variables|Default|GetPyramidLight) (Math|Float|Lerp (Variables|Default|GetPointLightIntensity) 0.0 Alpha)))